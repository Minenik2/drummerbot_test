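; Animation notify state for Sitri's drumstick animations that tells ABP_sitri_drumsticks when an animation is playing.
; On begin it casts the mesh's anim instance to that Blueprint and sets IsAnimationPlaying.
; On end it calls QueueState with cymbal, hihat and snare all false, clears the playing flag and prints a "reset state" debug string.
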(fn `Received_NotifyBegin`
  (params (MeshComp :type "SkeletalMeshComponent Object Reference") (Animation :type "AnimSequenceBase Object Reference") (TotalDuration :type "Float (single-precision)") (EventReference :type "AnimNotifyEventReference Structure (by ref)"))
  (returns (ReturnValue :type Boolean))
  (bind _asabp_sitri_drumsticks (cast `/Game/models/character/sitri/anims/ABP_sitri_drumsticks` (`SkeletalMeshComponent.GetAnimInstance` MeshComp)))
  (set `/Game/models/character/sitri/anims/ABP_sitri_drumsticks.isAnimationPlaying` true _asabp_sitri_drumsticks)
  (return false))

(fn `Received_NotifyEnd`
  (params (MeshComp :type "SkeletalMeshComponent Object Reference") (Animation :type "AnimSequenceBase Object Reference") (EventReference :type "AnimNotifyEventReference Structure (by ref)"))
  (returns (ReturnValue :type Boolean))
  (bind _asabp_sitri_drumsticks (cast `/Game/models/character/sitri/anims/ABP_sitri_drumsticks` (`SkeletalMeshComponent.GetAnimInstance` MeshComp)))
  (`/Game/models/character/sitri/anims/ABP_sitri_drumsticks.queueState` _asabp_sitri_drumsticks false false false false)
  (set `/Game/models/character/sitri/anims/ABP_sitri_drumsticks.isAnimationPlaying` false _asabp_sitri_drumsticks)
  (`KismetSystemLibrary.PrintString` null "reset state" true true (struct :`R` 1.0 :`G` 0.355408 :`B` 0.424788 :`A` 1.0))
  (return false))