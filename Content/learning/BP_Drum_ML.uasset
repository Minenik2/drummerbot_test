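; BP_Drum_ML is a physics drum, apparently a target for BP_BallAgent in a learning setup, that spawns at a random spot and yaw.
; ResetLocation, called on BeginPlay, reattaches the mesh, zeroes its velocities and moves the actor within a fixed area, raised by its box extent.
; A ball hit latches HasCollidedWithBall.
; When the ball's overlap ends, the drum clears that flag and sets HasCollidedWithDrum on the agent.
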(event `self.ReceiveBeginPlay`
  (`self.Reset Location`)
  (set `self.OriginalLocation` (`self.K2_GetActorLocation`)))

(event `self.ReceiveHit`
  (params (MyComp :type "PrimitiveComponent Object Reference") (Other :type "Actor Object Reference") (OtherComp :type "PrimitiveComponent Object Reference") (bSelfMoved :type Boolean) (HitLocation :type "Vector Structure") (HitNormal :type "Vector Structure") (NormalImpulse :type "Vector Structure") (Hit :type "HitResult Structure (by ref)"))
  (`KismetSystemLibrary.IsObjectOfSoftClass` (`ActorComponent.GetOwner` (`Actor.RootComponent` Other)) "/Game/learning/BP_BallAgent.BP_BallAgent_C"
    (:`True`
      (if (not (`self.hasCollidedWithBall`))
        (set `self.hasCollidedWithBall` true)
        (`KismetSystemLibrary.PrintString` "we've been hit!")))))

(event `self.ReceiveActorEndOverlap`
  (params (OtherActor :type "Actor Object Reference"))
  (`KismetSystemLibrary.IsObjectOfSoftClass` OtherActor "/Game/learning/BP_BallAgent.BP_BallAgent_C"
    (:`True`
      (set `self.hasCollidedWithBall` false)
      (bind _asbp_ball_agent (cast `/Game/learning/BP_BallAgent` (`ActorComponent.GetOwner` (`Actor.RootComponent` OtherActor))))
      (set `/Game/learning/BP_BallAgent.hasCollidedWithDrum` true _asbp_ball_agent))))

(fn `Reset Location`
  (`SceneComponent.K2_AttachToComponent` (`self.mesh`) (`self.DefaultSceneRoot`) "None" "KeepRelative" "KeepRelative" "KeepRelative" true)
  (`SceneComponent.K2_SetRelativeTransform` (`self.mesh`) (`KismetMathLibrary.MakeTransform` (0.0 0.0 32.0)) false true)
  (`self.K2_SetActorTransform` (`KismetMathLibrary.MakeTransform` (`KismetMathLibrary.MakeVector` (.x (`KismetMathLibrary.RandomPointInBoundingBox` (600.0 300.0 0.0) (300.0 150.0 0.0))) (.y (`KismetMathLibrary.RandomPointInBoundingBox` (600.0 300.0 0.0) (300.0 150.0 0.0))) (+ (.z (`KismetMathLibrary.RandomPointInBoundingBox` (600.0 300.0 0.0) (300.0 150.0 0.0))) (.z (`BoxComponent.BoxExtent` (`self.Box`))))) (`KismetMathLibrary.MakeRotator` 0.0 0.0 (`KismetMathLibrary.RandomFloatInRange` 0.0 360.0))))
  (`PrimitiveComponent.SetPhysicsLinearVelocity` (`self.mesh`) (0.0 0.0 0.0) false "None")
  (`PrimitiveComponent.SetPhysicsAngularVelocityInDegrees` (`self.mesh`) (0.0 0.0 0.0) false "None")
  (`KismetSystemLibrary.PrintString` (`KismetStringLibrary.Concat_StrStr` (`KismetStringLibrary.Conv_VectorToString` (`self.K2_GetActorLocation`)) " location spawned ") true true (struct :`R` 1.0 :`G` 0.286919 :`B` 0.398669 :`A` 1.0) 200.0))

(fn `UserConstructionScript`)