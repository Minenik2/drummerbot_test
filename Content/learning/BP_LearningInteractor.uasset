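; Learning Agents interactor that defines what BP_BallAgent ball agents observe and how their actions are applied.
; Observations hold the ball's location and forward direction plus its nearest drum's location, all relative to the ball mesh's own transform.
; Actions are a yaw value, set directly as actor rotation, and a nested X/Y movement pair with a large float scale, written to the agent's target action values.
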(fn `GatherAgentObservation`
  (params (InObservationObject :type "LearningAgentsObservationObject Object Reference") (AgentId :type Integer))
  (returns (OutObservationObjectElement :type "LearningAgentsObservationObjectElement Structure"))
  (locals (ObsActor :type "/Game/learning/BP_BallAgent Object Reference"))
  (bind _mesh (`/Game/learning/BP_BallAgent.mesh` (`local.ObsActor`)))
  (bind _returnvalue (`SceneComponent.K2_GetComponentToWorld` _mesh))
  (set `local.ObsActor` (`self.GetAgent` AgentId "/Game/learning/BP_BallAgent.BP_BallAgent_C"))
  (return (`LearningAgentsObservations.MakeStructObservation` (`local.InObservationObject`) (`|MakeMap` "ball" (`LearningAgentsObservations.MakeStructObservation` (`local.InObservationObject`) (`|MakeMap` "Location" (`LearningAgentsObservations.MakeLocationObservation` (`local.InObservationObject`) (`SceneComponent.K2_GetComponentLocation` _mesh) _returnvalue "LocationObservation" false null) "Direction" (`LearningAgentsObservations.MakeDirectionObservation` (`local.InObservationObject`) (`Actor.GetActorForwardVector` (`local.ObsActor`)) _returnvalue "DirectionObservation" false null) :!type "Name")) "drum" (`LearningAgentsObservations.MakeLocationObservation` (`local.InObservationObject`) (`SceneComponent.K2_GetComponentLocation` (`/Game/learning/BP_Drum_ML.mesh` (`/Game/learning/BP_BallAgent.NearestDrum` (`local.ObsActor`)))) (`SceneComponent.K2_GetComponentToWorld` (`/Game/learning/BP_BallAgent.mesh` (`local.ObsActor`))) "LocationObservation" false null) :!type "Name"))))

(fn `PerformAgentAction`
  (params (InActionObject :type "LearningAgentsActionObject Object Reference") (InActionObjectElement :type "LearningAgentsActionObjectElement Structure (by ref)") (AgentId :type Integer))
  (locals (ActActor :type "/Game/learning/BP_BallAgent Object Reference"))
  (bind _actactor (`local.ActActor`))
  (set `local.ActActor` (`self.GetAgent` AgentId "/Game/learning/BP_BallAgent.BP_BallAgent_C"))
  (bind _outelements (`LearningAgentsActions.GetStructAction` (`local.InActionObject`) (`local.InActionObjectElement`)))
  (`|ExecutionSequence`
    (:`then_0`
      (bind _outvalue (`LearningAgentsActions.GetFloatAction` (`local.InActionObject`) (`BlueprintMapLibrary.Map_Find` _outelements "Rotation") "FloatAction" false null))
      (`Actor.K2_SetActorRotation` (`local.ActActor`) (`KismetMathLibrary.MakeRotator` 0.0 0.0 _outvalue) false))
    (:`then_1`
      (bind _outelements_2 (`LearningAgentsActions.GetStructAction` (`local.InActionObject`) (`BlueprintMapLibrary.Map_Find` _outelements "Movement")))
      (`|ExecutionSequence`
        (:`then_0`
          (bind _outvalue_2 (`LearningAgentsActions.GetFloatAction` (`local.InActionObject`) (`BlueprintMapLibrary.Map_Find` _outelements_2 "XInput") "FloatAction" false null))
          (set `/Game/learning/BP_BallAgent.TargetActionValueX` _outvalue_2 _actactor))
        (:`then_1`
          (bind _outvalue_3 (`LearningAgentsActions.GetFloatAction` (`local.InActionObject`) (`BlueprintMapLibrary.Map_Find` _outelements_2 "YInput") "FloatAction" false null))
          (set `/Game/learning/BP_BallAgent.TargetActionValueY` _outvalue_3 _actactor))))))

(fn `SpecifyAgentAction`
  (params (InActionSchema :type "LearningAgentsActionSchema Object Reference"))
  (returns (OutActionSchemaElement :type "LearningAgentsActionSchemaElement Structure"))
  (return (`LearningAgentsActions.SpecifyStructAction` (`local.InActionSchema`) (`|MakeMap` "Rotation" (`LearningAgentsActions.SpecifyFloatAction` (`local.InActionSchema`)) "Movement" (`LearningAgentsActions.SpecifyStructAction` (`local.InActionSchema`) (`|MakeMap` "XInput" (`LearningAgentsActions.SpecifyFloatAction` (`local.InActionSchema`) 10000.0) "YInput" (`LearningAgentsActions.SpecifyFloatAction` (`local.InActionSchema`) 10000.0) :!type "Name")) :!type "Name"))))

(fn `SpecifyAgentObservation`
  (params (InObservationSchema :type "LearningAgentsObservationSchema Object Reference"))
  (returns (OutObservationSchemaElement :type "LearningAgentsObservationSchemaElement Structure"))
  (locals (NewLocalVar :type "LearningAgentsObservationObjectElement Structure"))
  (return (`LearningAgentsObservations.SpecifyStructObservation` (`local.InObservationSchema`) (`|MakeMap` "ball" (`LearningAgentsObservations.SpecifyStructObservation` (`local.InObservationSchema`) (`|MakeMap` "Location" (`LearningAgentsObservations.SpecifyLocationObservation` (`local.InObservationSchema`)) "Direction" (`LearningAgentsObservations.SpecifyDirectionObservation` (`local.InObservationSchema`)) :!type "Name")) "drum" (`LearningAgentsObservations.SpecifyLocationObservation` (`local.InObservationSchema`)) :!type "Name"))))