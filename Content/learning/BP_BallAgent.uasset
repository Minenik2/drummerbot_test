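; BP_BallAgent is a physics-driven ball that acts as a Learning Agents agent in a scene with drums.
; On BeginPlay it caches the nearest BP_Drum_ML and registers with the tagged LearningAgentsManager.
; Each tick it pushes its mesh with externally set X/Y action values and updates its distance to that cached drum.
; ResetToPoint clears actions and velocities, moves the mesh to a hard-coded start, and signals episode completion.
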(event `self.ReceiveBeginPlay`
  (`|ExecutionSequence`
    (:`then_0`
      (set `self.TargetActionValueY` 0.0)
      (set `self.TargetActionValueX` 0.0))
    (:`then_1`
      (bind _outactors (`GameplayStatics.GetAllActorsOfClass` "/Game/learning/BP_Drum_ML.BP_Drum_ML_C"))
      (bind (_distance _returnvalue) (`GameplayStatics.FindNearestActor` (`self.K2_GetActorLocation`) _outactors))
      (set `self.ClosestDistanceToDrum` _distance)
      (bind _asbp_drum_ml (cast `/Game/learning/BP_Drum_ML` _returnvalue))
      (set `self.NearestDrum` _asbp_drum_ml))
    (:`then_2`
      (bind _outactors_2 (`GameplayStatics.GetAllActorsWithTag` "LearningAgentsManager"))
      (for _array_element _outactors_2
        (bind _returnvalue_2 (`self.GetComponentByClass` _array_element "/Script/LearningAgents.LearningAgentsManager"))
        (`/Engine/EditorBlueprintResources/StandardMacros.IsValid` _returnvalue_2
          (:`Is Valid`
            (`LearningAgentsManager.AddAgent` _returnvalue_2 self)
            (set `self.FoundManager` true))))
      (if (not (`self.FoundManager`))
        (`KismetSystemLibrary.PrintString` "The agent could not find the learning agent manager. Make sure we did not forget to add one to the sequence")))))

(event `self.ReceiveTick`
  (params (DeltaSeconds :type "Float (single-precision)"))
  (`PrimitiveComponent.AddForce` (`self.mesh`) (`KismetMathLibrary.MakeVector` (`self.TargetActionValueX`) (`self.TargetActionValueY`)) "None" false)
  (`self.UpdateNearest`))

(fn `ResetToPoint`
  (bind _mesh (`self.mesh`))
  (set `self.TargetActionValueX` 0.0)
  (set `self.TargetActionValueY` 0.0)
  (`PrimitiveComponent.SetPhysicsLinearVelocity` _mesh (0.0 0.0 0.0) false "None")
  (`PrimitiveComponent.SetPhysicsAngularVelocityInDegrees` _mesh (0.0 0.0 0.0) false "None")
  (`SceneComponent.K2_SetWorldLocation` _mesh (731.781713 -217.397427 84.011211) false false)
  (`self.OnEpisodeCompleted`))

(fn `UpdateNearest`
  (set `self.ClosestDistanceToDrum` (`KismetMathLibrary.Vector_Distance` (`SceneComponent.K2_GetComponentLocation` (`self.mesh`)) (`SceneComponent.K2_GetComponentLocation` (`/Game/learning/BP_Drum_ML.mesh` (`self.NearestDrum`))))))

(fn `UserConstructionScript`)