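; BP_DrummerCharacter is a drummer character meant to animate drum hits in response to MIDI notes.
; On BeginPlay it binds playAnimation to the MIDI manager's note-played event and caches its drumsticks Animation Blueprint.
; A switch on note number would queue kick, snare, hi-hat or cymbal states on that AnimBP.
; That switch is disconnected and playAnimation is empty, so notes currently trigger no animation.
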(event `self.ReceiveBeginPlay`
  (add `/Game/blueprints/BP_MidiManager.onNotePlayed` (`self.MIDI_Manager`) (delegate `playAnimation`))
  (bind _asabp_sitri_drumsticks (cast `/Game/models/character/sitri/anims/ABP_sitri_drumsticks` (`SkeletalMeshComponent.GetAnimInstance` (`self.SkeletalMesh`)))))

(event `playAnimation`
  (params (noteInt :type Integer)))

(fn `UserConstructionScript`)