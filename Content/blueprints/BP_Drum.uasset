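; BP_Drum is a drum actor that plays audio and visually pulses when its Hit event is called.
; BeginPlay stores the original scale and creates a dynamic material instance on the drum mesh.
; Hit starts the sound and restarts a timeline whose alpha drives both the actor's scale, uniformly based on original X, and a clamped emissive material parameter.
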(event `self.ReceiveBeginPlay`
  (set `self.OriginalScale` (`self.GetActorScale3D`))
  (bind _returnvalue (`PrimitiveComponent.CreateDynamicMaterialInstance` (`self.DrumMesh`) 0 null "None"))
  (set `self.MID_Emissive` _returnvalue))

(event `Hit`
  (bind _originalscale_x (`KismetMathLibrary.BreakVector` (`self.OriginalScale`)))
  (`AudioComponent.Play` (`self.DrumAudio`) 0.0)
  (bind (_direction _alpha) (`Timeline|HitTimeline` :!via `PlayFromStart`)
    (:`Update`
      (bind _returnvalue (`KismetMathLibrary.Lerp` _originalscale_x (* _originalscale_x (`self.MaxScale`)) _alpha))
      (`self.SetActorScale3D` (`KismetMathLibrary.MakeVector` _returnvalue _returnvalue _returnvalue))
      (`MaterialInstanceDynamic.SetScalarParameterValue` (`self.MID_Emissive`) "Emissivness" (`KismetMathLibrary.FClamp` (* _alpha (`self.Emissive Amount`)) 0.1 10.0)))))

(fn `UserConstructionScript`)