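; Pawn that lets the player play a drum kit through Enhanced Input.
; On BeginPlay it adds the IMC_Drums mapping context to the local player's Enhanced Input subsystem.
; Input actions for kick, snare, hi-hat and cymbal each call Hit on the matching referenced drum piece.
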(event `self.ReceiveBeginPlay`
  (bind _asplayer_controller (cast `PlayerController` (`self.GetController`)))
  (`/Engine/EditorBlueprintResources/StandardMacros.IsValid` _asplayer_controller
    (:`Is Valid`
      (`EnhancedInputSubsystemInterface.AddMappingContext` (pcsubsystem `EnhancedInputLocalPlayerSubsystem` _asplayer_controller) "/Game/input/IMC_Drums.IMC_Drums" 0 (struct)))))

(event `EnhancedInput|/Game/input/IA_PlayKick`
  (params (ActionValue :type Boolean) (ElapsedSeconds :type "Float (double-precision)") (TriggeredSeconds :type "Float (double-precision)") (InputAction :type "InputAction Object Reference" :default "/Game/input/IA_PlayKick.IA_PlayKick"))
  (:`Triggered`
    (`/Game/blueprints/BP_Drum.Hit` (`self.BP_Drum_kick`))))

(event `EnhancedInput|/Game/input/IA_PlayCymbal`
  (params (ActionValue :type Boolean) (ElapsedSeconds :type "Float (double-precision)") (TriggeredSeconds :type "Float (double-precision)") (InputAction :type "InputAction Object Reference" :default "/Game/input/IA_PlayCymbal.IA_PlayCymbal"))
  (:`Triggered`
    (`/Game/blueprints/BP_Drum.Hit` (`self.BP_DRUM_Cymbal`))))

(event `EnhancedInput|/Game/input/IA_PlayHiHat`
  (params (ActionValue :type Boolean) (ElapsedSeconds :type "Float (double-precision)") (TriggeredSeconds :type "Float (double-precision)") (InputAction :type "InputAction Object Reference" :default "/Game/input/IA_PlayHiHat.IA_PlayHiHat"))
  (:`Triggered`
    (`/Game/blueprints/BP_Drum.Hit` (`self.BP_DRUM_HIHAT`))))

(event `EnhancedInput|/Game/input/IA_PlaySnare`
  (params (ActionValue :type Boolean) (ElapsedSeconds :type "Float (double-precision)") (TriggeredSeconds :type "Float (double-precision)") (InputAction :type "InputAction Object Reference" :default "/Game/input/IA_PlaySnare.IA_PlaySnare"))
  (:`Triggered`
    (`/Game/blueprints/BP_Drum.Hit` (`self.BP_DRUM_Snare`))))

(fn `UserConstructionScript`)